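; AchievementsBP is an actor that mirrors the player's run statistics, presumably for achievements, though it holds no unlock logic.
; Every Tick it casts the player pawn to TopDownCharacter and copies kills, waves survived and points, plus rounded game time.
; It then finds the first MyTheGamePlayerController through a per-frame GetAllActorsOfClass search and copies its bullet count.
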(event EventBeginPlay)

(event EventTick
  (params (DeltaSeconds :type Float%20%28single-precision%29))
  (bind _astop_down_character (Utilities|Casting|CastToTopDownCharacter (Game|GetPlayerCharacter 0)))
  (Variables|Default|SetkillCount (Variables|/Game/TopDownCPP/Blueprints/TopDownCharacter.TopDownCharacter_C|GetKills _astop_down_character))
  (Variables|Default|SetwaveCount (Variables|/Game/TopDownCPP/Blueprints/TopDownCharacter.TopDownCharacter_C|GetWavesSurvived _astop_down_character))
  (Variables|Default|SetscoreCount (Variables|/Game/TopDownCPP/Blueprints/TopDownCharacter.TopDownCharacter_C|GetPoints _astop_down_character))
  (Variables|Default|SettimeCount (Math|Float|Round (Utilities|Time|GetGameTimeinSeconds)))
  (bind _outactors (Actor|GetAllActorsOfClass "/Game/MyTheGamePlayerController.MyTheGamePlayerController_C"))
  (bind _asmy_the_game_player_controller (Utilities|Casting|CastToMyTheGamePlayerController (Utilities|Array|Get(acopy) _outactors)))
  (Variables|Default|SetbulletCount (Variables|/Game/MyTheGamePlayerController.MyTheGamePlayerController_C|GetbulletCount _asmy_the_game_player_controller)))

(fn ConstructionScript)